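; Game instance Blueprint that tracks player HP and coins and handles player death.
; HP events subtract or add fixed amounts, and IsTake updates coins, each broadcasting the result through an event dispatcher.
; When HP runs out, it calls PlayMontage on the player mesh, disables movement and input, and shows the WBP_Dead widget.
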(event Custom|HP-
  (bind _returnvalue (Game|GetPlayerCharacter 0))
  (bind _output_get (Variables|Default|SetHP (- (Variables|Default|GetHP) 5.0)))
  (Default|CallEDHP _output_get)
  (if (<= _output_get 0.0)
    (Animation|Montage|PlayMontage (Variables|/Script/Engine.Character|GetMesh _returnvalue) 0
      (:then
        (Pawn|Components|CharacterMovement|DisableMovement (Variables|/Script/Engine.Character|GetCharacterMovement _returnvalue))
        (Input|DisableInput (Game|GetPlayerController 0) 0)
        (bind _returnvalue_2 (UserInterface|CreateWidget "/Game/project/LVLUI/WBP/WBP_Dead.WBP_Dead_C"))
        (UserInterface|Viewport|AddtoViewport _returnvalue_2 0)))))

(event Custom|HP+
  (bind _output_get (Variables|Default|SetHP (+ (Variables|Default|GetHP) 5e+01)))
  (Default|CallEDHP _output_get))

(fn IsTake
  (params (Coins :type Float%20%28double-precision%29))
  (bind _output_get (Variables|Default|SetCoins (+ (Variables|Default|GetCoins) Coins)))
  (Default|CallEDCoins _output_get)
  (return _output_get))