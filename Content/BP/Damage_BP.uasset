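; Damage_BP is a hazard volume that damages actors implementing BPI_Damage when they enter its box.
; On begin overlap it applies DamageCharacter as base damage once and adds a WBP_DamageEffect widget to the viewport.
; On end overlap it sends DamageStopMessage through the interface and removes that widget.
; An unconnected BP_MyGI cast and HP call never runs.
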(event OnComponentBeginOverlap(Box)
  (params (OverlappedComponent :type Primitive%20Component%20Object%20Reference) (OtherActor :type Actor%20Object%20Reference) (OtherComp :type Primitive%20Component%20Object%20Reference) (OtherBodyIndex :type Integer) (bFromSweep :type Boolean) (SweepResult :type Hit%20Result%20Structure%20%28by%20ref%29))
  (if (Utilities|DoesObjectImplementInterface OtherActor "/Game/BP/Intefaces/BPI_Damage.BPI_Damage_C")
    (Game|Damage|ApplyDamage OtherActor (Variables|Default|GetDamageCharacter) 0 0)
    (bind _returnvalue (UserInterface|CreateWidget "/Game/project/LVLUI/WBP/WBP_DamageEffect.WBP_DamageEffect_C"))
    (UserInterface|Viewport|AddtoViewport _returnvalue 0)))

(event OnComponentEndOverlap(Box)
  (params (OverlappedComponent :type Primitive%20Component%20Object%20Reference) (OtherActor :type Actor%20Object%20Reference) (OtherComp :type Primitive%20Component%20Object%20Reference) (OtherBodyIndex :type Integer))
  (if (Utilities|DoesObjectImplementInterface OtherActor "/Game/BP/Intefaces/BPI_Damage.BPI_Damage_C")
    (Class|BPIDamageStop|DamageStop(Message) OtherActor)
    (Widget|RemovefromParent (stale OnComponentBeginOverlap(Box) _returnvalue))))

(event EventBeginPlay)

(event Collision|EventActorBeginOverlap
  (params (OtherActor :type Actor%20Object%20Reference)))

(event EventTick
  (params (DeltaSeconds :type Float%20%28single-precision%29)))

(fn ConstructionScript)